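; Patrol component for AI that hands out locations from a list of placed patrol point actors.
; GetNextPoint returns the current point's location, and CurrentPointFinish steps the index forward or backward according to the Reversing flag.
; When the index leaves the list, Loop restarts at the first point and Reverse flips direction from the end point.
; It prints an error when no valid point is found.
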(fn `CurrentPointFinish`
  (bind _currentpoint (`self.CurrentPoint`))
  (if (`self.Reversing`)
    (set `self.CurrentPoint` (- _currentpoint 1))
    (else
      (set `self.CurrentPoint` (+ _currentpoint 1)))))

(fn `GetNextPoint`
  (returns (NewParam :type "Vector Structure"))
  (bind _partolpoints (`self.PartolPoints`))
  (bind _currentpoint (`self.CurrentPoint`))
  (if (`KismetArrayLibrary.Array_IsValidIndex` _partolpoints _currentpoint)
    (return (`Actor.K2_GetActorLocation` (`|GetArrayItem` _partolpoints _currentpoint)))
    (else
      (switch `/Game/Dev/Waffle/Secret/AI/Task/PartolType` (`self.PartolType`)
        (:`NewEnumerator0`
          (bind _output_get (set `self.CurrentPoint` 0))
          (if (`KismetArrayLibrary.Array_IsValidIndex` (`self.PartolPoints`) _output_get)
            (return (`Actor.K2_GetActorLocation` (`|GetArrayItem` (`self.PartolPoints`) (`self.CurrentPoint`))))
            (else
              _)))
        (:`NewEnumerator1`
          (if (`self.Reversing`)
            (set `self.Reversing` false)
            (bind _output_get_2 (set `self.CurrentPoint` 0))
            (if (`KismetArrayLibrary.Array_IsValidIndex` (`self.PartolPoints`) _output_get_2)
              (return (`Actor.K2_GetActorLocation` (`|GetArrayItem` (`self.PartolPoints`) (`self.CurrentPoint`))))
              (else
                _))
            (else
              (set `self.Reversing` true)
              (bind _output_get_3 (set `self.CurrentPoint` (- (`self.CurrentPoint`) 1)))
              (if (`KismetArrayLibrary.Array_IsValidIndex` (`self.PartolPoints`) _output_get_3)
                (return (`Actor.K2_GetActorLocation` (`|GetArrayItem` (`self.PartolPoints`) (`self.CurrentPoint`))))
                (else
                  _))))))
      (`KismetSystemLibrary.PrintString` "Find No Partol point " true true (struct :`R` 1.0 :`G` 0.074642 :`A` 1.0)))))