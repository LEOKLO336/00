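; BP_KeyDoor is a door that opens when a player character carrying enough keys enters its overlap volume.
; On overlap, it casts to ThirdPersonCharacterHookTest1, compares NumberOfKeys with RequireNumberOfkeys and deducts that amount.
; It then plays the Doormovement timeline to set the door's relative location.
; The lerp's Alpha is fixed at zero, so the timeline's Movey output drives the position and TargetLocation has no effect.
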(event `self.Overlap.OnComponentBeginOverlap`
  (params (OverlappedComponent :type "PrimitiveComponent Object Reference") (OtherActor :type "Actor Object Reference") (OtherComp :type "PrimitiveComponent Object Reference") (OtherBodyIndex :type Integer) (bFromSweep :type Boolean) (SweepResult :type "HitResult Structure (by ref)"))
  (bind _requirenumberofkeys (`self.RequireNumberOfkeys`))
  (bind _asthird_person_character_hook_test_1 (cast `/Game/Dev/Yaya/ThirdPersonCharacterHookTest1` OtherActor))
  (bind _numberofkeys (`/Game/Dev/Yaya/ThirdPersonCharacterHookTest1.NumberOfKeys` _asthird_person_character_hook_test_1))
  (if (>= _numberofkeys _requirenumberofkeys)
    (set `/Game/Dev/Yaya/ThirdPersonCharacterHookTest1.NumberOfKeys` (- _numberofkeys _requirenumberofkeys) _asthird_person_character_hook_test_1)
    (bind (_direction _movey) (`Timeline|Doormovement`)
      (:`Update`
        (`SceneComponent.K2_SetRelativeLocation` (`self.Door`) (`KismetMathLibrary.VLerp` _movey (`self.TargetLocation`)) false false)))))

(fn `UserConstructionScript`)